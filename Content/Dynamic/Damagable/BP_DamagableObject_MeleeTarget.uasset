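; Damageable melee target, apparently a shield, that spins continuously on Z and damages any damageable actor that hits its mesh.
; BPCDamageSystem handles health and drives the death and hit events, with hits only printing debug text.
; Death briefly pauses the spin and boosts the dynamic material's emissive, while fractured geometry is hidden after a delay.
; The mesh starts hidden without collision until Respawn restores it and heals.
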(event OnComponentHit(StaticMesh)
  (params (HitComponent :type Primitive%20Component%20Object%20Reference) (OtherActor :type Actor%20Object%20Reference) (OtherComp :type Primitive%20Component%20Object%20Reference) (NormalImpulse :type Vector :default "0, 0, 0") (Hit :type Hit%20Result%20Structure%20%28by%20ref%29))
  ;[1 1 1] Hacer daño al personaje
  (if (Utilities|DoesObjectImplementInterface OtherActor "/Game/Dynamic/DamageSystem/BPI_Damagable.BPI_Damagable_C")
    (Class|BPIDamagable|TakeDamage(Message) OtherActor (Utilities|Struct|MakeS_DamageInfo 2e+01 "NewEnumerator1" "NewEnumerator2" false false (Math|Vector|MakeVector (* (.x (.impactpoint Hit)) 1e+01) (* (.y (.impactpoint Hit)) 1e+01) 0.0)))))

(event Custom|Death
  ;[1 1 1] Death
  (|CallParentFunction)
  (CallFunction|StopMovingUpandDown)
  (CallFunction|StopRotatingonZ)
  (Rendering|Material|SetScalarParameterValue (Variables|Default|GetMeshDynamicMaterial) "Emissive color 01 multiply" 2e+01 :!class /Script/Engine.MaterialInstanceDynamic)
  (Utilities|FlowControl|Delay 0.3)
  (CallFunction|RotateonZ)
  (Rendering|Material|SetScalarParameterValue (Variables|Default|GetMeshDynamicMaterial) "Emissive color 01 multiply" 1.0 :!class /Script/Engine.MaterialInstanceDynamic))

(event Custom|StopRotatingOnZ
  (bind _rotationbeforerotating (Variables|Default|GetRotationBeforeRotating))
  ;[1 1 1] Rotar en z
  (bind _zalpha (Timeline|RotateTimeline Stop)
    (:Update
      (Transformation|SetActorRotation (Math|Rotator|MakeRotator 0.0 0.0 (Math|Float|Lerp (.yaw _rotationbeforerotating) (+ (.yaw _rotationbeforerotating) 3.6e+02) _zalpha))))
    (:Finished
      (CallFunction|RotateonZ))))

(event Custom|Respawn
  (bind _staticmesh (Variables|Default|GetStaticMesh))
  ;[1 1 1] Respawn Shields
  (|CallParentFunction)
  (Collision|SetCollisionEnabled _staticmesh "QueryAndPhysics")
  (Rendering|SetVisibility _staticmesh true false)
  (Variables|/Game/Dynamic/DamageSystem/BPC_DamageSystem.BPC_DamageSystem_C|SetIsDead (Variables|Default|GetBPC_DamageSystem) false)
  (Default|Heal (Variables|Default|GetBPC_DamageSystem) 5e+01))

(event Custom|RotateOnZ
  ;[1 1 1] Rotar en z
  (Variables|Default|SetRotationBeforeRotating (Transformation|GetActorRotation))
  (bind _zalpha (Timeline|RotateTimeline PlayFromStart)
    (:Update
      (Transformation|SetActorRotation (Math|Rotator|MakeRotator 0.0 0.0 (Math|Float|Lerp (.yaw (Variables|Default|GetRotationBeforeRotating)) (+ (.yaw (Variables|Default|GetRotationBeforeRotating)) 3.6e+02) _zalpha))))
    (:Finished
      (CallFunction|RotateonZ))))

(event EventDamageResponse
  (params (DamageResponse :type E_DamageResponse%20Enum :default "NewEnumerator0") (HitLocation :type Vector :default "0, 0, 0"))
  (Development|PrintString "Has golpeado el escudo")
  (bind _health (CallFunction|GetCurrentHealth))
  (Development|PrintString (Utilities|String|ToString(Float) _health)))

(event Collision|EventActorBeginOverlap
  (params (OtherActor :type Actor%20Object%20Reference))
  (|CallParentFunction OtherActor) ; This node is disabled and will not be called.\nDrag off pins to build functionality.
)

(event EventTick
  (params (DeltaSeconds :type Float%20%28single-precision%29))
  (|CallParentFunction DeltaSeconds) ; This node is disabled and will not be called.\nDrag off pins to build functionality.
)

(event EventAddFracturedGeometry
  ;[1 1 1] Evento añadir geometria fracturada
  (bind _returnvalue (AddComponent|AddGeometryCollectionComponent false))
  (bind _output_get (Variables|Default|SetFracturedGeometryCollection _returnvalue))
  (Utilities|FlowControl|Delay 3.0)
  (Rendering|SetVisibility _output_get false false)
  (Collision|SetCollisionEnabled _output_get "NoCollision"))

(event EventBeginPlay
  (|CallParentFunction)
  (CallFunction|RotateonZ))

(fn ConstructionScript
  (bind _bpc_damagesystem (Variables|Default|GetBPC_DamageSystem))
  (bind _staticmesh (Variables|Default|GetStaticMesh))
  (|CallParentFunction)
  (bind _returnvalue (Rendering|Material|CreateDynamicMaterialInstance "/Game/Dynamic/StarterContent/Materials/M_Tech_Hex_Tile_Pulse_Inst.M_Tech_Hex_Tile_Pulse_Inst" "None" "None" :!class /Script/Engine.KismetMaterialLibrary))
  (bind _output_get (Variables|Default|SetMeshDynamicMaterial _returnvalue))
  (Rendering|Material|SetMaterial (Variables|Default|GetStaticMesh) 0 _output_get)
  (EventDispatchers|BindEventtoOnDeath _bpc_damagesystem (EventDispatchers|CreateEvent :!event Custom|Death))
  (EventDispatchers|BindEventtoOnDamageResponse _bpc_damagesystem (EventDispatchers|CreateEvent :!event DamageResponse))
  (Rendering|SetVisibility _staticmesh false false)
  (Collision|SetCollisionEnabled _staticmesh "NoCollision"))

(fn TakeDamage
  (params (DamageInfo :type S%20Damage%20Info%20Structure))
  (bind _wasdamaged (Default|TakeDamage (Variables|Default|GetBPC_DamageSystem) DamageInfo))
  (return _wasdamaged))

(fn Heal
  (params (Amount :type Float%20%28double-precision%29))
  (bind _newhealth (Default|Heal (Variables|Default|GetBPC_DamageSystem) Amount))
  (return _newhealth))

(fn GetMaxHealth
  (return (Variables|/Game/Dynamic/DamageSystem/BPC_DamageSystem.BPC_DamageSystem_C|GetMaxHealth (Variables|Default|GetBPC_DamageSystem))))

(fn GetCurrentHealth
  (return (Variables|/Game/Dynamic/DamageSystem/BPC_DamageSystem.BPC_DamageSystem_C|GetHealth (Variables|Default|GetBPC_DamageSystem))))