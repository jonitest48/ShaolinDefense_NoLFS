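; BP_DamagableObject is a breakable prop that serves as a shield piece for BP_TopDownEnemyBoss.
; TakeDamage forwards to BPCDamageSystem; on death, it requires a boss parent actor, calls BreakShield, then Break.
; Break swaps the mesh for a geometry collection, fractures it with strain field and radial force, plays sound, notifies OnBreak and destroys itself after a delay.
; Health getters and Heal are stubs; the vertical bobbing timeline is never started.
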(event Custom|Death
  (bind _asbp_top_down_enemy_boss (Utilities|Casting|CastToBP_TopDownEnemyBoss (Actor|GetParentActor)))
  (bind _output_get (Variables|Default|SetAs%20BP%20Top%20Down%20Enemy%20Boss _asbp_top_down_enemy_boss))
  (Default|BreakShield _output_get)
  (CallFunction|Break))

(event Custom|DamageResponse
  (params (DamageResponse :type E_DamageResponse%20Enum :default "NewEnumerator0") (HitLocation :type Vector)))

(event Custom|MoveUpAndDown)

(event Custom|StopMovingUpAndDown
  (bind _actorlocationbeforemoving (Variables|Default|GetActorLocationBeforeMoving))
  (bind _movezalpha (Timeline|MoveTimeline Stop)
    (:Update
      (Transformation|SetActorLocation (Math|Vector|MakeVector (.x _actorlocationbeforemoving) (.y _actorlocationbeforemoving) (Math|Float|Lerp (.z _actorlocationbeforemoving) (+ (.z (Variables|Default|GetInitialActorLocation)) (Variables|Default|GetMaxMoveOnZAxis)) _movezalpha)) false false))))

(event Custom|Break
  (Components|DestroyComponent (Variables|Default|GetStaticMesh))
  (Variables|Default|SetShouldMove false)
  (CallFunction|AddFracturedGeometry)
  (Class|FieldSystemComponent|ApplyPhysicsField (Variables|Default|GetFieldSystem) true "Field_ExternalClusterStrain" 0 (Field|SetRadialFalloff (Variables|Default|GetRadialFalloff) 1e+02 0.0 1.0 0.0 1e+02 (Transformation|GetActorLocation) "Field_FallOff_None"))
  (Components|Activation|Activate (Variables|Default|GetRadialForce) false)
  (Audio|PlaySoundatLocation (Variables|Default|GetBreakingSound) (Transformation|GetActorLocation) "0, 0, 0" 1.0 1.0 0.0 0 0 0 0)
  (Default|CallOnBreak self)
  (Utilities|FlowControl|Delay 3.0)
  (Actor|DestroyActor))

(event Custom|AddFracturedGeometry
  (bind _returnvalue (AddComponent|AddGeometryCollectionComponent false))
  (Variables|Default|SetFracturedGeometryCollection _returnvalue))

(event EventBeginPlay
  (Utilities|FlowControl|Delay (Math|Random|RandomFloat))
  (Variables|Default|SetInitialActorLocation (Transformation|GetActorLocation))
  (CallFunction|MoveUpandDown))

(event Collision|EventActorBeginOverlap
  (params (OtherActor :type Actor%20Object%20Reference)))

(event EventTick
  (params (DeltaSeconds :type Float%20%28single-precision%29)))

(fn ConstructionScript
  (bind _bpc_damagesystem (Variables|Default|GetBPC_DamageSystem))
  (EventDispatchers|BindEventtoOnDeath _bpc_damagesystem (EventDispatchers|CreateEvent :!event Custom|Death))
  (EventDispatchers|BindEventtoOnDamageResponse _bpc_damagesystem (EventDispatchers|CreateEvent :!event Custom|DamageResponse)))

(fn GetCurrentHealth
  (return 0.0))

(fn GetMaxHealth
  (return 0.0))

(fn Heal
  (params (Amount :type Float%20%28double-precision%29))
  (return 0.0))

(fn TakeDamage
  (params (DamageInfo :type S%20Damage%20Info%20Structure))
  (bind _wasdamaged (Default|TakeDamage (Variables|Default|GetBPC_DamageSystem)))
  (return _wasdamaged))