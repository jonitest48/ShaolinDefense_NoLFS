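; Base area-of-effect actor that finds pawns within a radius and reports each through the OnAOEOverlapActor dispatcher.
; Trigger, optionally run on BeginPlay, does a one-shot sphere or box overlap with debug drawing, optionally ignoring the instigator.
; Only the box branch binds FireDamage, which sends fixed damage via TakeDamageMessage, and it binds after each dispatch, so the first hit misses it.
; The HitTime delay timer is unconnected.
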(event Custom|SpawnAOESphere
  (if (Variables|Default|GetisSphere)
    (Rendering|Debug|DrawDebugSphere (Transformation|GetActorLocation) (Variables|Default|GetRadius) 12 "(R=1.000000,G=0.044597,B=0.979877,A=1.000000)" 2.0)
    (bind _outactors (Collision|SphereOverlapActors (Transformation|GetActorLocation) (Variables|Default|GetRadius) (Utilities|Array|MakeArray "ObjectTypeQuery3") 0 (select (Variables|Default|GetIgnoreInstigator) (Utilities|Array|MakeArray (Game|GetInstigator)) 0)))
    (for _array_element _outactors
      (Default|CallOnAOEOverlapActor _array_element)
      (Development|PrintString (Utilities|GetDisplayName _array_element)))
    (else
      ;[1 1 1] DañoFuego
      (Rendering|Debug|DrawDebugBox :Center (Transformation|GetActorLocation) :Extent (Math|Conversions|ToVector(Float) (Variables|Default|GetRadius)))
      (bind _outactors_2 (Collision|BoxOverlapActors (Transformation|GetActorLocation) (Math|Conversions|ToVector(Float) (Variables|Default|GetRadius)) (Utilities|Array|MakeArray "ObjectTypeQuery3") 0 (select (Variables|Default|GetIgnoreInstigator) (Utilities|Array|MakeArray (Game|GetInstigator)) 0) :!class /Script/Engine.KismetSystemLibrary))
      (for _array_element_2 _outactors_2
        (Default|CallOnAOEOverlapActor _array_element_2)
        (Development|PrintString (Utilities|GetDisplayName _array_element_2))
        (EventDispatchers|BindEventtoOnAOEOverlapActor (delegate Custom|FireDamage))))))

(event Custom|Trigger
  (CallFunction|SpawnAOESphere))

(event Custom|FireDamage
  (params (Actor :type Actor%20Object%20Reference))
  ;[1 1 1] DañoFuego
  (Class|BPIDamagable|TakeDamage(Message) Actor (Utilities|Struct|MakeS_DamageInfo 5.0 "NewEnumerator1" "NewEnumerator1")))

(event EventBeginPlay
  (if (Variables|Default|GetStartOnBeginPlay)
    (CallFunction|Trigger)))

(fn ConstructionScript)