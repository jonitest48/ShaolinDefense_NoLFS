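; BP_CurationDrop is a health pickup that spins in place and heals the player on contact.
; On BeginPlay, a looping timer fires every twentieth of a second to add yaw to the Cube component, producing the spin without Tick.
; When the player character overlaps the Cube, it sends HealMessage to that actor, clears the timer and destroys itself.
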(event OnComponentBeginOverlap(Cube)
  (params (OverlappedComponent :type Primitive%20Component%20Object%20Reference) (OtherActor :type Actor%20Object%20Reference) (OtherComp :type Primitive%20Component%20Object%20Reference) (OtherBodyIndex :type Integer) (bFromSweep :type Boolean) (SweepResult :type Hit%20Result%20Structure%20%28by%20ref%29))
  ;[1 1 1] Curar
  (if (== OtherActor (Game|GetPlayerCharacter 0))
    (Class|BPIDamagable|Heal(Message) OtherActor 5e+01)
    (Utilities|Time|ClearandInvalidateTimerbyHandle (Variables|Default|GetEventHandle))
    (Actor|DestroyActor)))

(event Custom|AddRotation
  (bind _cube (Variables|Default|GetCube))
  (bind _relativerotation (Variables|/Script/Engine.SceneComponent|GetRelativeRotation _cube))
  ;[1 1 1] Que gire
  (Transformation|SetRelativeRotation _cube (Math|Rotator|MakeRotator (.roll _relativerotation) (.pitch _relativerotation) (+ (.yaw _relativerotation) 1e+01)) false false))

(event EventBeginPlay
  ;[1 1 1] Que gire
  (bind _returnvalue (Utilities|Time|SetTimerbyEvent (delegate Custom|AddRotation) 0.05 true))
  (Variables|Default|SetEventHandle _returnvalue))

(fn ConstructionScript)