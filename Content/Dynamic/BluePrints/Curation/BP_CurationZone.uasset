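; BP_CurationZone is a healing zone that restores health to a BP_TopDownCharacter standing inside its box.
; Box overlap passes a DoOnce gate, reads the character's max health and starts a looping timer that sends fixed heal amounts via HealMessage.
; The timer stops and the gate resets when the returned value exceeds max health or a BP_TopDownCharacter leaves the box.
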(event OnComponentBeginOverlap(Box)
  (params (OverlappedComponent :type Primitive%20Component%20Object%20Reference) (OtherActor :type Actor%20Object%20Reference) (OtherComp :type Primitive%20Component%20Object%20Reference) (OtherBodyIndex :type Integer) (bFromSweep :type Boolean) (SweepResult :type Hit%20Result%20Structure%20%28by%20ref%29))
  (bind _asbp_top_down_character (Utilities|Casting|CastToBP_TopDownCharacter OtherActor))
  (Utilities|FlowControl|DoOnce false
    (:Completed
      (Development|PrintString "bien")
      (bind _maxhealth (Class|BPIDamagable|GetMaxHealth(Message) _asbp_top_down_character))
      (bind _returnvalue (Utilities|Time|SetTimerbyEvent (delegate Custom|HealLoop) 0.5 true))
      (Variables|Default|SetTimerHandler _returnvalue))))

(event OnComponentEndOverlap(Box)
  (params (OverlappedComponent :type Primitive%20Component%20Object%20Reference) (OtherActor :type Actor%20Object%20Reference) (OtherComp :type Primitive%20Component%20Object%20Reference) (OtherBodyIndex :type Integer))
  (Utilities|Casting|CastToBP_TopDownCharacter OtherActor)
  (Utilities|Time|ClearandInvalidateTimerbyHandle (Variables|Default|GetTimerHandler))
  (Utilities|FlowControl|DoOnce false) ; enters at Reset
)

(event Custom|HealLoop
  (bind _newhealth (Class|BPIDamagable|Heal(Message) (stale OnComponentBeginOverlap(Box) _asbp_top_down_character) 5.0))
  (if (not (<= _newhealth (stale OnComponentBeginOverlap(Box) _maxhealth)))
    (Utilities|Time|ClearandInvalidateTimerbyHandle (Variables|Default|GetTimerHandler))
    (Utilities|FlowControl|DoOnce false) ; enters at Reset
  ))

(fn ConstructionScript)