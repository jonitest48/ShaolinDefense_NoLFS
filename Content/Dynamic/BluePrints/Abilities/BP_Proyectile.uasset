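; BP_Proyectile is an ability projectile actor that damages enemies it overlaps and destroys itself after a short lifetime.
; Overlaps on Sphere1 skip player 0's character and send DamageInfo through BPI_Damagable to Enemy-tagged actors, recording each so it is hit only once.
; A BeginPlay timer fires Explosion, which only destroys the actor.
; Its own damage and health functions are stubs returning false or zero.
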(event OnComponentBeginOverlap(Sphere1)
  (params (OverlappedComponent :type Primitive%20Component%20Object%20Reference) (OtherActor :type Actor%20Object%20Reference) (OtherComp :type Primitive%20Component%20Object%20Reference) (OtherBodyIndex :type Integer) (bFromSweep :type Boolean) (SweepResult :type Hit%20Result%20Structure%20%28by%20ref%29))
  (bind _enemies (Variables|Default|GetEnemies))
  ;[1 1 1] Comprobar si tiene interfaz de daño implementada y si la tiene quitar vida
  (if (!= OtherActor (Game|GetPlayerCharacter 0))
    (if (and (Utilities|DoesObjectImplementInterface OtherActor "/Game/Dynamic/DamageSystem/BPI_Damagable.BPI_Damagable_C") (Actor|ActorHasTag OtherActor "Enemy"))
      (if (== (Utilities|Array|FindItem _enemies OtherActor) -1)
        (Utilities|Array|Add _enemies OtherActor)
        (Class|BPIDamagable|TakeDamage(Message) OtherActor (Variables|Default|GetDamage%20Info))))))

(event Custom|Explosion
  ;[1 1 1] Explosion FInal
  (Actor|DestroyActor))

(event EventBeginPlay
  ;[1 1 1] Spawn
  (Utilities|Time|SetTimerbyEvent (delegate Custom|Explosion) 0.5))

(fn ConstructionScript)

(fn TakeDamage
  (params (DamageInfo :type S%20Damage%20Info%20Structure))
  (return false))

(fn Heal
  (params (Amount :type Float%20%28double-precision%29))
  (return 0.0))

(fn GetMaxHealth
  (return 0.0))

(fn GetCurrentHealth
  (return 0.0))