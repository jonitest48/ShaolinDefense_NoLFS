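; Round manager that runs wave-based enemy rounds from the Rondas array, then spawns BP_TopDownEnemyBoss at its own transform once all are done.
; Each wave triggers CallSpawnMele and CallSpawnRanged through self-calling, delayed events, with another delay between waves.
; MuertedeEnemigo counts kills, and CheckNextRound compares them to the round's total, resetting counters and starting the next round after a pause.
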(event Custom|ManagerRondas
  (params (Ronda :type S%20Rounds%20Structure))
  ;[1 1 1] Sistema de Rondas
  (Development|PrintString "EMPIEZA LA RONDA" true true "(R=0.782126,G=1.000000,B=0.000000,A=1.000000)")
  (CallFunction|InvocarEnemigos))

(event Custom|ElegirRonda
  (bind _rondas (Variables|Default|GetRondas))
  (bind _rondaactual (Variables|Default|GetRondaActual))
  (bind _output (Utilities|Array|Get(acopy) _rondas _rondaactual))
  (bind (_tiempoentreoleadas _enemigosrangedoleada _totaloleadas _enemigosmeleoleada) (Utilities|Struct|BreakS_Rounds _output))
  ;[1 1 1] Elegir Nueva Ronda
  (if (< (Variables|Default|GetRondaActual) (Utilities|Array|Length (Variables|Default|GetRondas)))
    (Variables|Default|SettotalEnemiesInRound (+ (* _enemigosrangedoleada _totaloleadas) (* _enemigosmeleoleada _totaloleadas)))
    (CallFunction|ManagerRondas _output)
    (else
      (Game|SpawnActorfromClass "/Game/Dynamic/BluePrints/Enemies/BP_TopDownEnemyBoss.BP_TopDownEnemyBoss_C" (Transformation|GetActorTransform) "Undefined" "MultiplyWithRoot" 0 0)
      (Development|PrintString "RONDA DEL JEFE" true true "(R=1.000000,G=0.000000,B=0.779832,A=1.000000)"))))

(event Custom|InvocarEnemigos
  ;[1 1 1] Sistema de Rondas
  ;;[1 0.974 0.4423] Invocar Enemigos
  (CallFunction|InvocarMeles (stale Custom|ManagerRondas Ronda))
  (CallFunction|InvocarRangeds (stale Custom|ManagerRondas Ronda))
  (Utilities|FlowControl|Delay (.TiempoEntreOleadas (Utilities|Struct|BreakS_Rounds (stale Custom|ManagerRondas Ronda))))
  (bind _result (Math|Integer|IncrementInt (Variables|Default|GetOleadaActual))
    (:%20%20
      (if (< _result (.TotalOleadas (Utilities|Struct|BreakS_Rounds (stale Custom|ManagerRondas Ronda))))
        (CallFunction|InvocarEnemigos)
        (else
          (CallFunction|CheckNextRound))))))

(event Custom|Invocar%20Rangeds
  (params (Ronda :type S%20Rounds%20Structure))
  ;[1 1 1] Invocar Rangeds
  (Utilities|FlowControl|Delay 0.5)
  (Default|CallSpawnRanged)
  (bind _result (Math|Integer|IncrementInt (Variables|Default|GetRangedActual))
    (:%20%20
      (if (< _result (.EnemigosRangedOleada (Utilities|Struct|BreakS_Rounds Ronda)))
        (CallFunction|InvocarRangeds)
        (else
          (Variables|Default|SetRangedActual 0))))))

(event Custom|CheckNextRound
  ;[1 1 1] Comprobar si al acabar todas las oleadas se puede pasar a la siguiente ronda
  (Development|PrintString "COMPROBAR RONDAS" true true "(R=0.000000,G=1.000000,B=0.061501,A=1.000000)")
  (if (== (Variables|Default|GetenemiesKilled) (Variables|Default|GettotalEnemiesInRound))
    (Development|PrintString "RONDA ACANADA")
    (Variables|Default|SettotalEnemiesInRound 0)
    (Variables|Default|SetenemiesKilled 0)
    (Variables|Default|SetOleadaActual 0)
    (Variables|Default|SetMeleActual 0)
    (Variables|Default|SetRangedActual 0)
    (Math|Integer|IncrementInt (Variables|Default|GetRondaActual)
      (:%20%20
        (Utilities|FlowControl|Delay 1e+01)
        (CallFunction|ElegirRonda)))))

(event Custom|Invocar%20Meles
  (params (Ronda :type S%20Rounds%20Structure))
  ;[1 1 1] Invocar Meles
  (Utilities|FlowControl|Delay 0.5)
  (Default|CallSpawnMele)
  (bind _result (Math|Integer|IncrementInt (Variables|Default|GetMeleActual))
    (:%20%20
      (if (< _result (.EnemigosMeleOleada (Utilities|Struct|BreakS_Rounds Ronda)))
        (CallFunction|InvocarMeles)
        (else
          (Variables|Default|SetMeleActual 0))))))

(event Custom|Muerte%20de%20Enemigo
  ;[1 1 1] Cuando mata a un enemigo, comprobar el pasar de ronda
  (bind _result (Math|Integer|IncrementInt (Variables|Default|GetenemiesKilled))
    (:%20%20
      (Development|PrintString (Utilities|String|ToString(Integer) _result))
      (CallFunction|CheckNextRound))))

(event EventBeginPlay
  ;[1 1 1] Empezar
  (Utilities|FlowControl|Delay 3.0)
  (Utilities|FlowControl|Delay 3.0)
  (CallFunction|ElegirRonda))

(fn ConstructionScript)