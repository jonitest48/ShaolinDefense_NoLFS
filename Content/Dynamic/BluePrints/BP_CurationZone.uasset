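; BP_CurationZone is a healing area that restores health to a BP_TopDownCharacter standing inside its Cylinder volume.
; Beginning an overlap stores the character and starts a looping timer that calls its HealMessage at a fixed interval.
; The timer clears when the value returned by HealMessage reaches a threshold or when any overlap with the cylinder ends.
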(event OnComponentBeginOverlap(Cylinder)
  (params (OverlappedComponent :type Primitive%20Component%20Object%20Reference) (OtherActor :type Actor%20Object%20Reference) (OtherComp :type Primitive%20Component%20Object%20Reference) (OtherBodyIndex :type Integer) (bFromSweep :type Boolean) (SweepResult :type Hit%20Result%20Structure%20%28by%20ref%29))
  (bind _asbp_top_down_character (Utilities|Casting|CastToBP_TopDownCharacter OtherActor))
  (bind _returnvalue (Utilities|Time|SetTimerbyEvent (delegate Custom|HealLoop) 0.5 true))
  (Variables|Default|SetTimerHandler _returnvalue))

(event OnComponentEndOverlap(Cylinder)
  (params (OverlappedComponent :type Primitive%20Component%20Object%20Reference) (OtherActor :type Actor%20Object%20Reference) (OtherComp :type Primitive%20Component%20Object%20Reference) (OtherBodyIndex :type Integer))
  (Utilities|Time|ClearandInvalidateTimerbyHandle (Variables|Default|GetTimerHandler)))

(event Custom|HealLoop
  (bind _newhealth (Class|BPIDamagable|Heal(Message) (stale OnComponentBeginOverlap(Cylinder) _asbp_top_down_character) 5.0))
  (if (>= _newhealth 5e+01)
    (Utilities|Time|ClearandInvalidateTimerbyHandle (Variables|Default|GetTimerHandler))))

(fn ConstructionScript)