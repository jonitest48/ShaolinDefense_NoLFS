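; BP_DashShadow is a short-lived decoy that pulls non-ranged enemies off their tower target.
; Sphere overlap stores the actor as Enemy and retargets a BP_TopDownEnemy to the shadow, while the ranged retarget branch is left disconnected.
; After a delay, only the last stored Enemy, ranged or not, is sent back to its TowerTarget before the shadow destroys itself.
; Health getters read BPCDamageSystem, but Heal and TakeDamage are inert stubs.
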(event OnComponentBeginOverlap(Sphere)
  (params (OverlappedComponent :type Primitive%20Component%20Object%20Reference) (OtherActor :type Actor%20Object%20Reference) (OtherComp :type Primitive%20Component%20Object%20Reference) (OtherBodyIndex :type Integer) (bFromSweep :type Boolean) (SweepResult :type Hit%20Result%20Structure%20%28by%20ref%29))
  (Variables|Default|SetEnemy OtherActor)
  (CallFunction|ChangeTargettoDummy))

(event Custom|Change%20Target%20To%20Dummy
  (bind _enemy (Variables|Default|GetEnemy))
  (bind _asbp_top_down_enemy_ranged (Utilities|Casting|CastToBP_TopDownEnemyRanged _enemy)
    (:CastFailed
      (bind _asbp_top_down_enemy (Utilities|Casting|CastToBP_TopDownEnemy _enemy))
      (Variables|/Game/Dynamic/BluePrints/Enemies/BP_TopDownEnemy.BP_TopDownEnemy_C|SetTarget _asbp_top_down_enemy self)
      (Default|MoveEnemytoActor _asbp_top_down_enemy))))

(event Custom|Change%20Target%20To%20Tower
  (bind _enemy (Variables|Default|GetEnemy))
  (bind _asbp_top_down_enemy_ranged (Utilities|Casting|CastToBP_TopDownEnemyRanged _enemy)
    (:then
      (Variables|/Game/Dynamic/BluePrints/Enemies/BP_TopDownEnemyRanged.BP_TopDownEnemyRanged_C|SetTarget _asbp_top_down_enemy_ranged (Variables|/Game/Dynamic/BluePrints/Enemies/BP_TopDownEnemyRanged.BP_TopDownEnemyRanged_C|GetTowerTarget _asbp_top_down_enemy_ranged))
      (Default|MoveEnemytoActor _asbp_top_down_enemy_ranged))
    (:CastFailed
      (bind _asbp_top_down_enemy (Utilities|Casting|CastToBP_TopDownEnemy _enemy))
      (Variables|/Game/Dynamic/BluePrints/Enemies/BP_TopDownEnemy.BP_TopDownEnemy_C|SetTarget _asbp_top_down_enemy (Variables|/Game/Dynamic/BluePrints/Enemies/BP_TopDownEnemy.BP_TopDownEnemy_C|GetTowerTarget _asbp_top_down_enemy))
      (Default|MoveEnemytoActor _asbp_top_down_enemy))))

(event EventBeginPlay
  (Utilities|FlowControl|Delay 5.0)
  (CallFunction|ChangeTargettoTower)
  (Actor|DestroyActor))

(fn ConstructionScript)

(fn GetCurrentHealth
  (return (Variables|/Game/Dynamic/DamageSystem/BPC_DamageSystem.BPC_DamageSystem_C|GetHealth (Variables|Default|GetBPC_DamageSystem))))

(fn GetMaxHealth
  (return (Variables|/Game/Dynamic/DamageSystem/BPC_DamageSystem.BPC_DamageSystem_C|GetMaxHealth (Variables|Default|GetBPC_DamageSystem))))

(fn Heal
  (params (Amount :type Float%20%28double-precision%29))
  (return 0.0))

(fn TakeDamage
  (params (DamageInfo :type S%20Damage%20Info%20Structure))
  (return false))