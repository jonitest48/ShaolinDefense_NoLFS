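; Ranged enemy spawner that, on a T key press, releases an enemy from the BPCEnemyPoolRanged pool.
; It detaches the pooled enemy at the current index, enables its collision, teleports it to the spawner and calls MoveEnemyToActor on it.
; The index advances round-robin through the pool, reusing actors instead of spawning new ones.
; The unhide call targets the spawner itself, not the pooled enemy.
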(event Input|KeyboardEvents|T
  (params (Key :type Key%20Structure :default "None"))
  (bind _bpc_enemypoolranged (Variables|Default|GetBPC_EnemyPoolRanged))
  (bind _rangedpool (Variables|/Game/Dynamic/BluePrints/Enemy-Pools/BPC_EnemyPoolRanged.BPC_EnemyPoolRanged_C|GetRangedPool _bpc_enemypoolranged))
  (bind _returnvalue (Utilities|Array|Length _rangedpool))
  (:Pressed
    (if (> _returnvalue 0)
      (Variables|Default|SetMaxPool _returnvalue)
      (Utilities|IsValid (Utilities|Array|Get(acopy) _rangedpool (Variables|Default|GetRangedIndex))
        (:Is%20Valid
          (Transformation|DetachFromActor (Utilities|Array|Get(acopy) _rangedpool (Variables|Default|GetRangedIndex)) "KeepWorld" "KeepWorld" "KeepWorld")
          (Collision|SetActorEnableCollision (Utilities|Array|Get(acopy) _rangedpool (Variables|Default|GetRangedIndex)) true)
          (Rendering|SetActorHiddenInGame false)
          (Transformation|SetActorLocation (Utilities|Array|Get(acopy) _rangedpool (Variables|Default|GetRangedIndex)) (Transformation|GetActorLocation) false false)
          (Default|MoveEnemytoActor (Utilities|Array|Get(acopy) _rangedpool (Variables|Default|GetRangedIndex)))
          (bind _result (Math|Integer|IncrementInt (Variables|Default|GetRangedIndex))
            (:%20%20
              (bind _output_get (Variables|Default|SetRangedIndex _result))
              (if (== _output_get (Variables|Default|GetMaxPool))
                (Variables|Default|SetRangedIndex 0)))))))))

(fn ConstructionScript)