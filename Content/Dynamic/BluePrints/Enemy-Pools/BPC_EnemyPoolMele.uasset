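; Actor component that pre-spawns a pool of melee or ranged enemies for its owner and recycles them on death.
; After a one-second delay at BeginPlay, it picks the class from the enemy type, spawns the enemies attached to the owner and binds their death events.
; Deaths return enemies to the owner, deactivate them through BPI_Enemy and notify BP_RoundManager.
; Older melee-only pooling logic remains, disconnected.
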(event Custom|Mele%20Death
  (params (Enemy :type BP%20Top%20Down%20Enemy%20Object%20Reference))
  (bind _returnvalue (Components|GetOwner))
  (Rendering|SetActorHiddenInGame Enemy false)
  (Transformation|SetActorLocation Enemy (Transformation|GetActorLocation _returnvalue) false false)
  (Collision|SetActorEnableCollision Enemy false)
  (Transformation|AttachActorToActor Enemy _returnvalue "None" "KeepWorld" "KeepWorld" "KeepWorld" true))

(event Custom|Enemy%20Death
  (params (Enemy :type Actor%20Object%20Reference))
  (bind _returnvalue (Components|GetOwner))
  ;[1 1 1] Evento que cambia la localizacion el denemigo
  (Development|PrintString "MUERTO" true true "(R=1.000000,G=0.000000,B=0.070149,A=1.000000)")
  (Transformation|SetActorLocation Enemy (Transformation|GetActorLocation _returnvalue) false false)
  (Transformation|AttachActorToActor Enemy _returnvalue "None" "KeepWorld" "KeepWorld" "KeepWorld" true)
  (if (Utilities|DoesObjectImplementInterface Enemy "/Game/Dynamic/BluePrints/Enemies/EnemyElements/BPI_Enemy.BPI_Enemy_C")
    (Class|BPIEnemy|DeActivate(Message) Enemy)
    (Default|MuerteDeEnemigo (Variables|Default|GetRoundManager))))

(event Custom|Bind%20Event%20To%20Enemy%20Death
  (params (Enemy :type Actor%20Object%20Reference))
  (switch string (Variables|Default|GetEnemyTypeBC)
    (:Melee
      (bind _asbp_top_down_enemy (Utilities|Casting|CastToBP_TopDownEnemy Enemy))
      (EventDispatchers|BindEventtoOnMeleDeath _asbp_top_down_enemy (delegate Custom|On%20Mele%20Death%20Call)))
    (:Ranged
      (bind _asbp_top_down_enemy_ranged (Utilities|Casting|CastToBP_TopDownEnemyRanged Enemy))
      (EventDispatchers|BindEventtoOnRangedDeath _asbp_top_down_enemy_ranged (delegate Custom|On%20Ranged%20Death%20Call)))))

(event Custom|On%20Mele%20Death%20Call
  (params (Enemy :type BP%20Top%20Down%20Enemy%20Object%20Reference))
  (CallFunction|EnemyDeath Enemy))

(event Custom|On%20Ranged%20Death%20Call
  (params (Ranged :type BP%20Top%20Down%20Enemy%20Ranged%20Object%20Reference))
  (CallFunction|EnemyDeath Ranged))

(event EventBeginPlay
  (bind _enemytypebc (Variables|Default|GetEnemyTypeBC))
  (bind _returnvalue (Actor|GetActorOfClass "/Game/Dynamic/BluePrints/RoundSystem/BP_RoundManager.BP_RoundManager_C"))
  (Variables|Default|SetRoundManager _returnvalue)
  (Utilities|FlowControl|Delay 1.0)
  (Development|PrintString _enemytypebc)
  (CallFunction|SetEnemyClass _enemytypebc)
  (for _index (range 0 (Variables|Default|GetTotalEnemies))
    (bind _returnvalue_2 (Game|SpawnActorfromClass (Variables|Default|GetEnemyClass) (Math|Transform|MakeTransform (Transformation|GetActorLocation (Components|GetOwner)) "0, 0, 0" "1.000000,1.000000,1.000000") "AlwaysSpawn" "MultiplyWithRoot" 0 0))
    (bind _returnvalue_3 (Transformation|AttachActorToActor _returnvalue_2 (Components|GetOwner) "None" "KeepWorld" "KeepWorld" "KeepWorld" true))
    (if _returnvalue_3
      (Utilities|Array|Add (Variables|Default|GetEnemyPool) _returnvalue_2)
      (CallFunction|BindEventtoEnemyDeath _returnvalue_2))))

(fn SetEnemyClass
  (params (EnemyType :type String))
  (switch string EnemyType
    (:Melee
      (Variables|Default|SetEnemyClass "/Game/Dynamic/BluePrints/Enemies/BP_TopDownEnemy.BP_TopDownEnemy_C"))
    (:Ranged
      (Variables|Default|SetEnemyClass "/Game/Dynamic/BluePrints/Enemies/BP_TopDownEnemyRanged.BP_TopDownEnemyRanged_C"))))