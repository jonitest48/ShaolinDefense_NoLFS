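; Actor component that builds an object pool of BP_TopDownEnemyRanged enemies for its owning actor.
; On BeginPlay it spawns TotalEnemies-driven instances at the owner's location, disables their collision, attaches them, fills RangedPool and binds each death event.
; On death, an enemy is hidden rather than destroyed, offset locally by the owner's location and reattached.
; Spawned enemies start unhidden, and this graph has no logic for reactivating pooled enemies.
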(event Custom|RangedDeath
  (params (Ranged :type BP%20Top%20Down%20Enemy%20Ranged%20Object%20Reference))
  (bind _returnvalue (Components|GetOwner))
  (Rendering|SetActorHiddenInGame Ranged true)
  (Transformation|AddActorLocalOffset Ranged (Transformation|GetActorLocation _returnvalue) false false)
  (Transformation|AttachActorToActor Ranged _returnvalue "None" "KeepWorld" "KeepWorld" "KeepWorld" true))

(event EventBeginPlay
  (for _index (range 0 (Variables|Default|GetTotalEnemies))
    (bind _returnvalue (Game|SpawnActorfromClass "/Game/Dynamic/BluePrints/Enemies/BP_TopDownEnemyRanged.BP_TopDownEnemyRanged_C" (Math|Transform|MakeTransform (Transformation|GetActorLocation (Components|GetOwner)) "0, 0, 0" "1.000000,1.000000,1.000000") "AlwaysSpawn" "MultiplyWithRoot" 0 0))
    (Rendering|SetActorHiddenInGame _returnvalue false)
    (Collision|SetActorEnableCollision _returnvalue false)
    (Transformation|AttachActorToActor _returnvalue (Components|GetOwner) "None" "KeepWorld" "KeepWorld" "KeepWorld" true)
    (if true
      (Utilities|Array|Add (Variables|Default|GetRangedPool) 0)
      (EventDispatchers|BindEventtoOnRangedDeath _returnvalue (delegate Custom|RangedDeath)))))