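; BP_MeleSpawner activates pooled melee enemies at its own location when the round manager requests a spawn.
; On BeginPlay it binds SpawnEnemy to BP_RoundManager's melee spawn event.
; Each spawn takes the current entry from BPCEnemyPoolMele's pool, detaches it, re-enables collision and visibility, marks it active, moves it to the spawner and starts its movement.
; A wrapping index cycles through the pool round-robin without checking whether that enemy is already active.
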(event Custom|SpawnEnemy
  (bind _bpc_enemypoolmele (Variables|Default|GetBPC_EnemyPoolMele))
  (bind _melepool (Variables|/Game/Dynamic/BluePrints/Enemy-Pools/BPC_EnemyPoolMele.BPC_EnemyPoolMele_C|GetMelePool _bpc_enemypoolmele))
  (bind _returnvalue (Utilities|Array|Length _melepool))
  ;[1 1 1] Spawnear / Activar Enemigos
  (Development|PrintString "Invocar")
  (if (> _returnvalue 0)
    (Variables|Default|SetMaxPool _returnvalue)
    (Utilities|IsValid (Utilities|Array|Get(acopy) _melepool (Variables|Default|GetMeleIndex))
      (:Is%20Valid
        (Transformation|DetachFromActor (Utilities|Array|Get(acopy) _melepool (Variables|Default|GetMeleIndex)) "KeepWorld" "KeepWorld" "KeepWorld")
        (Collision|SetActorEnableCollision (Utilities|Array|Get(acopy) _melepool (Variables|Default|GetMeleIndex)) true)
        (Rendering|SetActorHiddenInGame (Utilities|Array|Get(acopy) _melepool (Variables|Default|GetMeleIndex)) false)
        (Variables|/Game/Dynamic/BluePrints/Enemies/BP_TopDownEnemy.BP_TopDownEnemy_C|SetisActive? (Utilities|Array|Get(acopy) _melepool (Variables|Default|GetMeleIndex)) true)
        (Transformation|SetActorLocation (Utilities|Array|Get(acopy) _melepool (Variables|Default|GetMeleIndex)) (Transformation|GetActorLocation) false false)
        (Default|MoveEnemytoActor (Utilities|Array|Get(acopy) _melepool (Variables|Default|GetMeleIndex)))
        (bind _result (Math|Integer|IncrementInt (Variables|Default|GetMeleIndex))
          (:%20%20
            (bind _output_get (Variables|Default|SetMeleIndex _result))
            (if (== _output_get (Variables|Default|GetMaxPool))
              (Variables|Default|SetMeleIndex 0))))))))

(event EventBeginPlay
  (bind _returnvalue (Actor|GetActorOfClass "/Game/Dynamic/BluePrints/RoundSystem/BP_RoundManager.BP_RoundManager_C"))
  (EventDispatchers|BindEventtoSpawnMele _returnvalue (delegate Custom|SpawnEnemy)))

(fn ConstructionScript)