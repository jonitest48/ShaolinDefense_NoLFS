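; BP_don is an actor scaffold for a damageable object, with a BPCDamageSystem component and no active gameplay logic.
; The construction script binds a delegate to the component's OnDamageResponse; the auto-generated DamageResponse and HitLocation handler is empty.
; GetCurrentHealth, GetMaxHealth, Heal and TakeDamage are stubs returning zero or false, without forwarding to the component.
; The event graph contains only disabled default events.
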(event EventBeginPlay)

(event Collision|EventActorBeginOverlap
  (params (OtherActor :type Actor%20Object%20Reference)))

(event EventTick
  (params (DeltaSeconds :type Float%20%28single-precision%29)))

(fn ConstructionScript
  (EventDispatchers|BindEventtoOnDamageResponse (Variables|Default|GetBPC_DamageSystem) (EventDispatchers|CreateEvent :!event BPDonAutoGenFunc)))

(fn BPDonAutoGenFunc
  (params (DamageResponse :type E_DamageResponse%20Enum :default "NewEnumerator0") (HitLocation :type Vector)))

(fn GetCurrentHealth
  (return 0.0))

(fn GetMaxHealth
  (return 0.0))

(fn Heal
  (params (Amount :type Float%20%28double-precision%29))
  (return 0.0))

(fn TakeDamage
  (params (DamageInfo :type S%20Damage%20Info%20Structure))
  (return false))