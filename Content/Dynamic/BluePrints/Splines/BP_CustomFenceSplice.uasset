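; Spline-driven fence Blueprint that builds fence panels and posts along its spline in the Construction Script, with no runtime logic.
; It steps along the spline by SegmentLength, bending a FenceBody spline mesh across each interval, with tangents clamped to segment length and a small fixed local X offset.
; A FencePost is placed at each step's start, also as a spline mesh component but only positioned, not fitted to the curve.
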(event EventBeginPlay)

(event Collision|EventActorBeginOverlap
  (params (OtherActor :type Actor%20Object%20Reference)))

(event EventTick
  (params (DeltaSeconds :type Float%20%28single-precision%29)))

(fn ConstructionScript
  (bind _spline (Variables|Default|GetSpline))
  (for _index (range 0 (Math|Float|Truncate (/ (Spline|GetSplineLength (Variables|Default|GetSpline)) (Variables|Default|GetSegmentLength))))
    (bind _returnvalue (AddComponent|AddSplineMeshComponent false))
    (Components|StaticMesh|SetStaticMesh _returnvalue (Variables|Default|GetFenceBody))
    (Transformation|SetRelativeTransform _returnvalue (Variables|Default|GetFenceBodyTransform) false false)
    (SplineMesh|SetStartandEnd _returnvalue (+ (Spline|GetLocationatDistanceAlongSpline _spline (* _index (Variables|Default|GetSegmentLength)) "Local") "10.000000,0.000000,0.000000") (Math|Vector|ClampVectorSize (Spline|GetTangentatDistanceAlongSpline _spline (* _index (Variables|Default|GetSegmentLength)) "Local") 0.0 (Variables|Default|GetSegmentLength)) (+ (Spline|GetLocationatDistanceAlongSpline _spline (* (+ _index 1) (Variables|Default|GetSegmentLength)) "Local") "10.000000,0.000000,0.000000") (Math|Vector|ClampVectorSize (Spline|GetTangentatDistanceAlongSpline _spline (* (+ _index 1) (Variables|Default|GetSegmentLength)) "Local") 0.0 (Variables|Default|GetSegmentLength)) true :!class /Script/Engine.SplineMeshComponent)
    (bind _returnvalue_2 (AddComponent|AddSplineMeshComponent false))
    (Components|StaticMesh|SetStaticMesh _returnvalue_2 (Variables|Default|GetFencePost))
    (Transformation|SetRelativeTransform _returnvalue_2 (Variables|Default|GetFencePostTranform) false false)
    (Transformation|SetRelativeLocation _returnvalue_2 (Spline|GetLocationatDistanceAlongSpline (Variables|Default|GetSpline) (* _index (Variables|Default|GetSegmentLength)) "Local") false false)))